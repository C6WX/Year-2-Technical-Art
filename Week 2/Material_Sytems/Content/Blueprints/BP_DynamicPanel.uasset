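; BP_DynamicPanel is a panel actor whose cube material responds to a character entering or leaving its box trigger.
; On BeginPlay it creates a dynamic material instance from the cube's material and assigns it back.
; Character overlap plays a timeline that lerps a named scalar parameter from 0 to 1.
; Ending overlap reverses the timeline from its end, so a partial fade jumps to the end before reversing.
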(event OnComponentBeginOverlap(Box)
  (params (OverlappedComponent :type Primitive%20Component%20Object%20Reference) (OtherActor :type Actor%20Object%20Reference) (OtherComp :type Primitive%20Component%20Object%20Reference) (OtherBodyIndex :type Integer) (bFromSweep :type Boolean) (SweepResult :type Hit%20Result%20Structure%20%28by%20ref%29))
  (Utilities|Casting|CastToCharacter OtherActor)
  (bind _lerpcontribution (Timeline|LerpMaterialValueTimeline Play)
    (:Update
      (Rendering|Material|SetScalarParameterValue (Variables|Default|GetDynamicMaterialReferance) (Variables|Default|GetParameter%20Name) (Math|Float|Lerp 0.0 1.0 _lerpcontribution) :!class /Script/Engine.MaterialInstanceDynamic))))

(event OnComponentEndOverlap(Box)
  (params (OverlappedComponent :type Primitive%20Component%20Object%20Reference) (OtherActor :type Actor%20Object%20Reference) (OtherComp :type Primitive%20Component%20Object%20Reference) (OtherBodyIndex :type Integer))
  (Utilities|Casting|CastToCharacter OtherActor)
  (bind _lerpcontribution (Timeline|LerpMaterialValueTimeline ReverseFromEnd)
    (:Update
      (Rendering|Material|SetScalarParameterValue (Variables|Default|GetDynamicMaterialReferance) (Variables|Default|GetParameter%20Name) (Math|Float|Lerp 0.0 1.0 _lerpcontribution) :!class /Script/Engine.MaterialInstanceDynamic))))

(event EventBeginPlay
  ;[1 1 1] Create Material
  (bind _returnvalue (Rendering|Material|CreateDynamicMaterialInstance (Rendering|Material|GetMaterial (Variables|Default|GetCube) 0) "None" "None" :!class /Script/Engine.KismetMaterialLibrary))
  (bind _output_get (Variables|Default|SetDynamicMaterialReferance _returnvalue))
  (Rendering|Material|SetMaterial (Variables|Default|GetCube) 0 _output_get))

(fn ConstructionScript)