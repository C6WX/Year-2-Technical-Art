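; Global controller Blueprint that cycles the level between day and night by writing light, fog and rain scalars to MPC_GlobalEffects.
; Day, also run at BeginPlay, and Night call each other after fixed Delays, forming an endless loop.
; IA_ChangeTime branches on TimeOfDay to switch phase, though "Night" is only set after Night's delay, immediately before Day resets it.
; Tick copies LightIntensity from the collection to the DirectionalLight.
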(event Custom|Night
  ;[1 1 1] Night
  (Rendering|Material|SetScalarParameterValue "/Game/Materials/MPC/MPC_GlobalEffects.MPC_GlobalEffects" "LightIntensity" 1.0 :!class /Script/Engine.KismetMaterialLibrary)
  (Rendering|Material|SetScalarParameterValue "/Game/Materials/MPC/MPC_GlobalEffects.MPC_GlobalEffects" "FogDensity" 0.0 :!class /Script/Engine.KismetMaterialLibrary)
  (Rendering|Material|SetScalarParameterValue "/Game/Materials/MPC/MPC_GlobalEffects.MPC_GlobalEffects" "RainAmount" 1e+02 :!class /Script/Engine.KismetMaterialLibrary)
  (Utilities|FlowControl|Delay 5.0)
  (Variables|Default|SetTimeOfDay "Night")
  (CallFunction|Day))

(event Custom|Day
  ;[1 1 1] Day
  (Rendering|Material|SetScalarParameterValue "/Game/Materials/MPC/MPC_GlobalEffects.MPC_GlobalEffects" "LightIntensity" 3.0 :!class /Script/Engine.KismetMaterialLibrary)
  (Rendering|Material|SetScalarParameterValue "/Game/Materials/MPC/MPC_GlobalEffects.MPC_GlobalEffects" "FogDensity" 1e+02 :!class /Script/Engine.KismetMaterialLibrary)
  (Rendering|Material|SetScalarParameterValue "/Game/Materials/MPC/MPC_GlobalEffects.MPC_GlobalEffects" "RainAmount" 0.0 :!class /Script/Engine.KismetMaterialLibrary)
  (Variables|Default|SetTimeOfDay "Day")
  (Utilities|FlowControl|Delay 5.0)
  (CallFunction|Night))

(event Input|EnhancedActionEvents|EnhancedInputActionIA_ChangeTime
  (params (ActionValue :type Boolean) (ElapsedSeconds :type Float%20%28double-precision%29) (TriggeredSeconds :type Float%20%28double-precision%29) (InputAction :type Input%20Action%20Object%20Reference :default "/Game/Blueprints/IA_ChangeTime.IA_ChangeTime"))
  ;[1 1 1] Change Time Of Day
  (if (Utilities|Enum|Equal(Enum) (Variables|Default|GetTimeOfDay) "Day")
    (CallFunction|Night)
    (elif (Utilities|Enum|Equal(Enum) (Variables|Default|GetTimeOfDay) "Night")
      (CallFunction|Day))))

(event EventBeginPlay
  ;[1 1 1] Day
  (Rendering|Material|SetScalarParameterValue "/Game/Materials/MPC/MPC_GlobalEffects.MPC_GlobalEffects" "LightIntensity" 3.0 :!class /Script/Engine.KismetMaterialLibrary)
  (Rendering|Material|SetScalarParameterValue "/Game/Materials/MPC/MPC_GlobalEffects.MPC_GlobalEffects" "FogDensity" 1e+02 :!class /Script/Engine.KismetMaterialLibrary)
  (Rendering|Material|SetScalarParameterValue "/Game/Materials/MPC/MPC_GlobalEffects.MPC_GlobalEffects" "RainAmount" 0.0 :!class /Script/Engine.KismetMaterialLibrary)
  (Variables|Default|SetTimeOfDay "Day")
  (Utilities|FlowControl|Delay 5.0)
  (CallFunction|Night))

(event EventTick
  (params (DeltaSeconds :type Float%20%28single-precision%29))
  ;[1 1 1] Light Intensity
  (bind _returnvalue (Actor|GetActorOfClass "/Script/Engine.DirectionalLight"))
  (bind _returnvalue_2 (Rendering|Material|GetScalarParameterValue "/Game/Materials/MPC/MPC_GlobalEffects.MPC_GlobalEffects" "LightIntensity" :!class /Script/Engine.KismetMaterialLibrary))
  (Rendering|Components|Light|SetIntensity (Variables|/Script/Engine.Light|GetLightComponent _returnvalue) _returnvalue_2))

(fn ConstructionScript)